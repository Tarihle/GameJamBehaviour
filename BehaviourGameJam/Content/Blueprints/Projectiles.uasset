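; Projectile actor that kills the third-person player character on hit and destroys itself two seconds after spawning.
; An IRMode event shows the actor and enables its mesh collision when on, and hides it and disables collision when off.
; Mesh hits cast the other actor to BP_ThirdPersonCharacter_Cube and call its Death function.
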(event `self.ReceiveBeginPlay`
  (`KismetSystemLibrary.Delay` 2.0)
  (`self.K2_DestroyActor`))

(event `IRMode`
  (params (`On/Off` :type Boolean))
  (`self.SetActorHiddenInGame` (not `On/Off`))
  (if `On/Off`
    (`PrimitiveComponent.SetCollisionEnabled` (`self.StaticMesh`) "QueryAndPhysics")
    (else
      (`PrimitiveComponent.SetCollisionEnabled` (`self.StaticMesh`) "NoCollision"))))

(event `self.StaticMesh.OnComponentHit`
  (params (HitComponent :type "PrimitiveComponent Object Reference") (OtherActor :type "Actor Object Reference") (OtherComp :type "PrimitiveComponent Object Reference") (NormalImpulse :type "Vector Structure") (Hit :type "HitResult Structure (by ref)"))
  (bind _asbp_third_person_character_cube (cast `/Game/ThirdPerson/Blueprints/BP_ThirdPersonCharacter_Cube` OtherActor))
  (`/Game/ThirdPerson/Blueprints/BP_ThirdPersonCharacter_Cube.Death` _asbp_third_person_character_cube))

(fn `UserConstructionScript`)