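; Laser hazard actor whose beam kills the cube third-person character on hit.
; Tick shows the beam and enables collision only while IR mode is on or OnRayHit fired, clearing that flag each frame so ray hits must repeat.
; While active, it either sweeps in yaw or, without a rotation angle, slides along its local Y, reversing at angle or height limits.
; BeginPlay sets beam size and height.
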(event `self.ReceiveBeginPlay`
  (`SceneComponent.SetWorldScale3D` (`self.Beam`) (`KismetMathLibrary.MakeVector` (`self.BeamSize_X`) (`self.BeamSize_Y`) (`self.BeamSize`)))
  (`SceneComponent.K2_SetRelativeLocation` (`self.Beam`) (`KismetMathLibrary.MakeVector` 0.0 0.0 (`self.BeamHeight`)) false false))

(event `Rotate`
  (bind (_returnvalue_roll _returnvalue_pitch _returnvalue_yaw) (`KismetMathLibrary.BreakRotator` (`self.K2_GetActorRotation`)))
  ;[1 1 1] Rotate
  (if (`self.Reverse`)
    (`self.K2_AddActorLocalRotation` (`KismetMathLibrary.MakeRotator` 0.0 0.0 -1.0))
    (else
      (`self.K2_AddActorLocalRotation` (`KismetMathLibrary.MakeRotator` 0.0 0.0 1.0))))
  (if (>= (`KismetMathLibrary.Abs` _returnvalue_yaw) (`self.Rotation Angle`))
    (set `self.Reverse` (not (`self.Reverse`)))))

(event `self.ReceiveTick`
  (params (DeltaSeconds :type "Float (single-precision)"))
  (if (or (`self.Activated`) (`self.IROn`))
    (`PrimitiveComponent.SetCollisionEnabled` (`self.Beam`) "QueryAndPhysics")
    (`SceneComponent.SetHiddenInGame` (`self.Beam`) false false)
    (set `self.Activated` false)
    (if (!= (`self.Rotation Angle`) 0.0)
      (`self.Rotate`)
      (elif (!= (`self.DeltaHeight`) 0.0)
        (`self.Move`)))
    (else
      (`PrimitiveComponent.SetCollisionEnabled` (`self.Beam`) "NoCollision")
      (`SceneComponent.SetHiddenInGame` (`self.Beam`) true false))))

(event `OnRayHit`
  (set `self.Activated` true))

(event `self.Beam.OnComponentHit`
  (params (HitComponent :type "PrimitiveComponent Object Reference") (OtherActor :type "Actor Object Reference") (OtherComp :type "PrimitiveComponent Object Reference") (NormalImpulse :type "Vector Structure") (Hit :type "HitResult Structure (by ref)"))
  (bind _asbp_third_person_character_cube (cast `/Game/ThirdPerson/Blueprints/BP_ThirdPersonCharacter_Cube` OtherActor))
  (`/Game/ThirdPerson/Blueprints/BP_ThirdPersonCharacter_Cube.Death` _asbp_third_person_character_cube))

(event `Move`
  (bind (_relativelocation_x _relativelocation_y _relativelocation_z) (`KismetMathLibrary.BreakVector` (`SceneComponent.RelativeLocation` (`self.Beam`))))
  (bind (_relativelocation_x_2 _relativelocation_y_2 _relativelocation_z_2) (`KismetMathLibrary.BreakVector` (`SceneComponent.RelativeLocation` (`self.Beam`))))
  (if (`self.Reverse`)
    (`SceneComponent.K2_AddLocalOffset` (`self.Beam`) (`KismetMathLibrary.MakeVector` 0.0 -1.0) false false)
    (else
      (`SceneComponent.K2_AddLocalOffset` (`self.Beam`) (`KismetMathLibrary.MakeVector` 0.0 1.0) false false)))
  (if (or (> _relativelocation_z_2 (+ (`self.BeamHeight`) (`self.DeltaHeight`))) (< _relativelocation_z (- (`self.BeamHeight`) (`self.DeltaHeight`))))
    (set `self.Reverse` (not (`self.Reverse`)))))

(event `self.CapsuleBeam.OnComponentBeginOverlap`
  (params (OverlappedComponent :type "PrimitiveComponent Object Reference") (OtherActor :type "Actor Object Reference") (OtherComp :type "PrimitiveComponent Object Reference") (OtherBodyIndex :type Integer) (bFromSweep :type Boolean) (SweepResult :type "HitResult Structure (by ref)")))

(event `IRMode`
  (params (`On/Off` :type Boolean))
  (set `self.IROn` `On/Off`))

(fn `UserConstructionScript`)