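; Dispenser actor that repeatedly spawns projectiles at its root transform while its IR flag is on.
; BeginPlay starts SpawnProjectile, a self-repeating Delay loop paced by ShootingDelay.
; After each delay it either spawns the Projectiles class and re-calls itself, or loops back to the delay when IROn is false.
; The IRMode event sets IROn, so the loop keeps polling while firing is off.
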(event `self.ReceiveBeginPlay`
  (`self.SpawnProjectile`))

(event `SpawnProjectile`
  (`KismetSystemLibrary.Delay` (`self.ShootingDelay`) :!label _label)
  (if (`self.IROn`)
    (`|SpawnActorFromClass` "/Game/Blueprints/Projectiles.Projectiles_C" (`SceneComponent.K2_GetComponentToWorld` (`self.DefaultSceneRoot`)) "Undefined" "MultiplyWithRoot" null null)
    (`self.SpawnProjectile`)
    (else
      (goto _label))))

(event `IRMode`
  (params (`On/Off` :type Boolean))
  (set `self.IROn` `On/Off`))

(fn `UserConstructionScript`)