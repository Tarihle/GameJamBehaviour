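; Spike trap that alternately rises and lowers, killing the third-person cube character on a SpikeMesh hit.
; Tick accumulates time only on frames following a ray hit or while IR mode is on, firing a FlipFlop between up and down timelines every two seconds.
; Both meshes move by offsets from SpikeMesh's current location.
; IRMode swaps mesh visibility and toggles IRSpike collision, but never re-enables SpikeMesh collision once disabled.
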(event `self.ReceiveTick`
  (params (DeltaSeconds :type "Float (single-precision)"))
  (if (or (`self.Activated`) (`self.IROn`))
    (set `self.Activated` false)
    (bind _output_get (set `self.AccTick` (+ DeltaSeconds (`self.AccTick`))))
    (if (>= _output_get 2.0)
      (`self.PicotiPicota`)
      (set `self.AccTick` 0.0))))

(event `PicotiPicota`
  (bind _returnvalue (`SceneComponent.K2_GetComponentLocation` (`self.SpikeMesh`)))
  (bind _returnvalue_2 (`SceneComponent.K2_GetComponentLocation` (`self.SpikeMesh`)))
  (`/Engine/EditorBlueprintResources/StandardMacros.FlipFlop`
    (:`A`
      (bind (_direction _spiky) (`Timeline|SpikeUp` :!via `PlayFromStart`)
        (:`Update`
          (bind _returnvalue_3 (`KismetMathLibrary.VLerp` _returnvalue_2 (+ _returnvalue_2 (0.0 0.0 5.0)) _spiky))
          (`SceneComponent.K2_SetWorldLocation` (`self.SpikeMesh`) _returnvalue_3 false false)
          (`SceneComponent.K2_SetWorldLocation` (`self.IRSpike`) _returnvalue_3 false false))))
    (:`B`
      (bind (_direction_2 _spiky_2) (`Timeline|Timeline` :!via `PlayFromStart`)
        (:`Update`
          (bind _returnvalue_4 (`KismetMathLibrary.VLerp` _returnvalue (+ _returnvalue (0.0 0.0 -5.0)) _spiky_2))
          (`SceneComponent.K2_SetWorldLocation` (`self.SpikeMesh`) _returnvalue_4 false false)
          (`SceneComponent.K2_SetWorldLocation` (`self.IRSpike`) _returnvalue_4 false false))))))

(event `IRMode`
  (params (`On/Off` :type Boolean))
  (set `self.IROn` `On/Off`)
  (`SceneComponent.SetHiddenInGame` (`self.IRSpike`) (not `On/Off`) false)
  (`SceneComponent.SetHiddenInGame` (`self.SpikeMesh`) `On/Off` false)
  (if `On/Off`
    (`PrimitiveComponent.SetCollisionEnabled` (`self.IRSpike`) "QueryAndPhysics")
    (`PrimitiveComponent.SetCollisionEnabled` (`self.SpikeMesh`) "NoCollision")
    (else
      (`PrimitiveComponent.SetCollisionEnabled` (`self.IRSpike`) "NoCollision"))))

(event `OnRayHit`
  (set `self.Activated` true))

(event `self.SpikeMesh.OnComponentHit`
  (params (HitComponent :type "PrimitiveComponent Object Reference") (OtherActor :type "Actor Object Reference") (OtherComp :type "PrimitiveComponent Object Reference") (NormalImpulse :type "Vector Structure") (Hit :type "HitResult Structure (by ref)"))
  (bind _asbp_third_person_character_cube (cast `/Game/ThirdPerson/Blueprints/BP_ThirdPersonCharacter_Cube` OtherActor))
  (`/Game/ThirdPerson/Blueprints/BP_ThirdPersonCharacter_Cube.Death` _asbp_third_person_character_cube))

(event `self.Box.OnComponentBeginOverlap`
  (params (OverlappedComponent :type "PrimitiveComponent Object Reference") (OtherActor :type "Actor Object Reference") (OtherComp :type "PrimitiveComponent Object Reference") (OtherBodyIndex :type Integer) (bFromSweep :type Boolean) (SweepResult :type "HitResult Structure (by ref)")))

(fn `UserConstructionScript`)